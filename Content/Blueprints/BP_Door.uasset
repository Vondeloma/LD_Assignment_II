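; BP_Door is a key-locked sliding door that opens once for the player.
; When the player character overlaps the Box with HaveKey set on ThirdPersonCharacter, the trigger is destroyed and the mesh changes material.
; The OpenDoor timeline then moves the mesh toward the Scene component's relative location, easing from its current position on each update rather than a cached start.
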(event OnComponentBeginOverlap(Box)
  (params (OverlappedComponent :type Primitive%20Component%20Object%20Reference) (OtherActor :type Actor%20Object%20Reference) (OtherComp :type Primitive%20Component%20Object%20Reference) (OtherBodyIndex :type Integer) (bFromSweep :type Boolean) (SweepResult :type Hit%20Result%20Structure%20%28by%20ref%29))
  (if (== OtherActor (Game|GetPlayerCharacter 0))
    (bind _asthird_person_character (Utilities|Casting|CastToThirdPersonCharacter OtherActor))
    (if (Variables|/Game/ThirdPersonBP/Blueprints/ThirdPersonCharacter.ThirdPersonCharacter_C|GetHaveKey _asthird_person_character)
      (Components|DestroyComponent (Variables|Default|GetBox))
      (Rendering|Material|SetMaterial (Variables|Default|GetStaticMesh) 0 "/Engine/VREditor/BasicMeshes/MI_Cube_4.MI_Cube_4")
      (bind _opendoor (Timeline|OpenDoor PlayFromStart)
        (:Update
          (Transformation|SetRelativeLocation (Variables|Default|GetStaticMesh) (Math|Interpolation|Ease "Linear" _opendoor (Variables|/Script/Engine.SceneComponent|GetRelativeLocation (Variables|Default|GetStaticMesh)) (Variables|/Script/Engine.SceneComponent|GetRelativeLocation (Variables|Default|GetScene))) false false))))))

(fn ConstructionScript)