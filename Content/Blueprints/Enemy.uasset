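; Patrolling stealth enemy that catches the player on sight and triggers their teleport-to-checkpoint message.
; A timeline ping-pongs the capsule between its start and a Scene component's location, pausing and turning the mesh at each end.
; While the player overlaps the detection Box, Tick line-traces toward them against pawns and static world, so cover can block detection.
; An Alarm material shows whether the player is out of range, in range or spotted.
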(event OnComponentBeginOverlap(Box)
  (params (OverlappedComponent :type Primitive%20Component%20Object%20Reference) (OtherActor :type Actor%20Object%20Reference) (OtherComp :type Primitive%20Component%20Object%20Reference) (OtherBodyIndex :type Integer) (bFromSweep :type Boolean) (SweepResult :type Hit%20Result%20Structure%20%28by%20ref%29))
  ;[1 1 1] Check if player is within "Detection Area"
  (if (== OtherActor (Game|GetPlayerCharacter 0))
    (Variables|Default|SetPlayerInRange true)
    (Rendering|Material|SetMaterial (Variables|Default|GetAlarm) 0 "/Engine/EditorMaterials/WidgetMaterial_Current.WidgetMaterial_Current")))

(event OnComponentEndOverlap(Box)
  (params (OverlappedComponent :type Primitive%20Component%20Object%20Reference) (OtherActor :type Actor%20Object%20Reference) (OtherComp :type Primitive%20Component%20Object%20Reference) (OtherBodyIndex :type Integer))
  ;[1 1 1] Check if player is within "Detection Area"
  (if (== OtherActor (Game|GetPlayerCharacter 0))
    (Variables|Default|SetPlayerInRange false)
    (Rendering|Material|SetMaterial (Variables|Default|GetAlarm) 0 "/Engine/EditorMaterials/WidgetMaterial.WidgetMaterial")))

(event EventBeginPlay
  (bind _mesh (Variables|Character|GetMesh))
  ;[1 1 1] Start patroling
  (Variables|Default|SetStartPos (Transformation|GetWorldLocation (Variables|Collision|GetCapsuleComponent)))
  (Variables|Default|SetEndPos (Transformation|GetWorldLocation (Variables|Default|GetScene)))
  (bind _patrol (Timeline|Patroling PlayFromStart)
    (:Update
      (Transformation|SetRelativeLocation (Variables|Collision|GetCapsuleComponent) (Math|Vector|Lerp(Vector) (Variables|Default|GetStartPos) (Variables|Default|GetEndPos) _patrol) false false))
    (:Finished
      (if (Variables|Default|GetPatrolFinished)
        (Variables|Default|SetPatrolFinished false)
        (Utilities|FlowControl|Delay 1.0)
        (Transformation|SetRelativeRotation _mesh (Variables|Default|GetWantedRotationOnReversPatrol) false false)
        (Timeline|Patroling PlayFromStart)
        (else
          (Variables|Default|SetPatrolFinished true)
          (Utilities|FlowControl|Delay 1.0)
          (Transformation|SetRelativeRotation _mesh "0,90.000000, 0" false false)
          (Timeline|Patroling ReverseFromEnd))))))

(event EventTick
  (params (DeltaSeconds :type Float%20%28single-precision%29))
  (bind _returnvalue (Game|GetPlayerCharacter 0))
  (bind _capsulecomponent (Variables|Collision|GetCapsuleComponent))
  (bind _returnvalue_2 (Transformation|GetWorldLocation _capsulecomponent))
  (bind _capsulecomponent_2 (Variables|/Script/Engine.Character|GetCapsuleComponent _returnvalue))
  (bind _returnvalue_3 (Transformation|GetWorldLocation _capsulecomponent_2))
  ;[1 1 1] Tick Event, look for player
  (if (Variables|Default|GetPlayerInRange)
    (bind (_outhit _returnvalue_4) (Collision|LineTraceForObjects (Math|Vector|MakeVector (.x _returnvalue_2) (.y _returnvalue_2) (+ (.z _returnvalue_2) 8e+01)) (Math|Vector|MakeVector (.x _returnvalue_3) (.y _returnvalue_3) (+ (.z _returnvalue_3) 45.0)) (Utilities|Array|MakeArray "ObjectTypeQuery3" "ObjectTypeQuery1") false 0 "ForDuration"))
    (if _returnvalue_4
      (if (== (.HitActor (Collision|BreakHitResult _outhit)) (Game|GetPlayerCharacter 0))
        (Rendering|Material|SetMaterial (Variables|Default|GetAlarm) 0 "/Engine/EditorMaterials/WidgetMaterial_X.WidgetMaterial_X")
        (Class|INTPlayer|TeleporttoCheckpoint(Message) (Game|GetPlayerCharacter 0))
        (else
          (Rendering|Material|SetMaterial (Variables|Default|GetAlarm) 0 "/Engine/EditorMaterials/WidgetMaterial_Current.WidgetMaterial_Current"))))))

(fn ConstructionScript)